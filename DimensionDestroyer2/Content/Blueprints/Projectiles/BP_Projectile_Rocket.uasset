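; BP_Projectile_Rocket is a rocket projectile that damages actors it overlaps and destroys itself after its lifetime.
; On BeginPlay it caches the player character, then waits out LifeTime as a stopgap against too many projectiles in the level.
; The capsule overlap applies BaseDamage to any actor except that player, without destroying the rocket.
; Health-based destruction logic exists but is disconnected, so incoming damage has no effect.
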(event `self.ReceiveBeginPlay`
  ;[1 1 1] Temporary solution from having too much bullets on the level (can also put invisible wall at corner of level and destroy on impact too)
  (bind _asbp_player_character (cast `/Game/Blueprints/Player/BP_PlayerCharacter` (`GameplayStatics.GetPlayerCharacter` 0)))
  (set `self.Character` _asbp_player_character)
  (`KismetSystemLibrary.Delay` (`self.LifeTime`))
  (`self.K2_DestroyActor`))

(event `self.Capsule Collider.OnComponentBeginOverlap`
  (params (OverlappedComponent :type "PrimitiveComponent Object Reference") (OtherActor :type "Actor Object Reference") (OtherComp :type "PrimitiveComponent Object Reference") (OtherBodyIndex :type Integer) (bFromSweep :type Boolean) (SweepResult :type "HitResult Structure (by ref)"))
  (if (not (== OtherActor (`self.Character`)))
    (`GameplayStatics.ApplyDamage` OtherActor (`self.BaseDamage`))))

(event `self.ReceiveAnyDamage`
  (params (Damage :type "Float (single-precision)") (DamageType :type "DamageType Object Reference") (InstigatedBy :type "Controller Object Reference") (DamageCauser :type "Actor Object Reference")))

(fn `UserConstructionScript`)