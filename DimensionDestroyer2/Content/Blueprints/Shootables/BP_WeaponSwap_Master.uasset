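; BP_WeaponSwap_Master is a shootable base Blueprint for weapon swap objects, showing the weapon's name on a text render.
; BeginPlay caches the player character and sets that text from WeaponSwapName.
; AnyDamage lowers health clamped between zero and one, then at zero waits briefly and calls SetPlayerWeapon.
; SetPlayerWeapon is empty here, apparently left for child Blueprints to implement the actual swap.
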(event `self.ReceiveBeginPlay`
  (bind _asbp_player_character (cast `/Game/Blueprints/Player/BP_PlayerCharacter` (`GameplayStatics.GetPlayerCharacter` 0)))
  (set `self.Character` _asbp_player_character)
  (`TextRenderComponent.K2_SetText` (`self.TextRender`) (`KismetTextLibrary.Conv_StringToText` (`self.WeaponSwapName`))))

(event `self.ReceiveAnyDamage`
  (params (Damage :type "Float (single-precision)") (DamageType :type "DamageType Object Reference") (InstigatedBy :type "Controller Object Reference") (DamageCauser :type "Actor Object Reference"))
  (bind _output_get (set `self.CurrentHealth` (`KismetMathLibrary.FClamp` (- (`self.CurrentHealth`) Damage))))
  (if (== _output_get 0.0)
    (`KismetSystemLibrary.Delay` 1.0)
    (`self.SetPlayerWeapon`)))

(event `SetPlayerWeapon`)

(fn `UserConstructionScript`)