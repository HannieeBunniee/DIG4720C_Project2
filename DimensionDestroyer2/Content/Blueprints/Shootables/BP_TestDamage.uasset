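; Test actor that takes damage and displays its remaining health as text.
; Tick writes CurrentHealth to a TextRender component every frame.
; AnyDamage subtracts the damage, clamps health to a fixed range, and destroys the actor when it reaches zero.
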(event `self.ReceiveBeginPlay`)

(event `self.ReceiveTick`
  (params (DeltaSeconds :type "Float (single-precision)"))
  (`TextRenderComponent.K2_SetText` (`self.TextRender`) (`KismetTextLibrary.Conv_DoubleToText` (`self.CurrentHealth`) "HalfToEven")))

(event `self.ReceiveAnyDamage`
  (params (Damage :type "Float (single-precision)") (DamageType :type "DamageType Object Reference") (InstigatedBy :type "Controller Object Reference") (DamageCauser :type "Actor Object Reference"))
  (bind _output_get (set `self.CurrentHealth` (`KismetMathLibrary.FClamp` (- (`self.CurrentHealth`) Damage) 0.0 1000.0)))
  (if (== _output_get 0.0)
    (`self.K2_DestroyActor`)))

(fn `UserConstructionScript`)