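; BP_LevelManager drives enemy spawning for the level.
; On BeginPlay it gathers all BP_Enemy_SpawnPoint actors, then a looping timer calls SpawnEnemy on a random one at the TimeBetweenNextEnemySpawn interval.
; A minutes-and-seconds countdown that would show UI_GameOver and pause the game at zero is present but disconnected, so Tick does nothing.
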(event `self.ReceiveBeginPlay`
  ;[1 1 1] Spawn enemy at random set point
  (bind _outactors (`GameplayStatics.GetAllActorsOfClass` "/Game/Blueprints/WaveManagement/BP_Enemy_SpawnPoint.BP_Enemy_SpawnPoint_C"))
  ;;[1 1 1] Time til next enemy spawn
  (set `self.Spawner list` _outactors)
  (`KismetSystemLibrary.K2_SetTimerDelegate` (delegate `ActivateSpawner`) (`self.Time between next enemy spawn`) true))

(event `ActivateSpawner`
  (bind _spawner_list (`self.Spawner list`))
  ;[1 1 1] Spawn enemy at random set point
  ;;[1 1 1] Get random Spawn point
  (`/Game/Blueprints/WaveManagement/BP_Enemy_SpawnPoint.SpawnEnemy` (`|GetArrayItem` _spawner_list (`KismetMathLibrary.RandomIntegerInRange` 0 (- (`KismetArrayLibrary.Array_Length` _spawner_list) 1)))))

(event `self.ReceiveTick`
  (params (DeltaSeconds :type "Float (single-precision)"))
  ;[1 1 1] Timer counting down
)

(fn `UserConstructionScript`)