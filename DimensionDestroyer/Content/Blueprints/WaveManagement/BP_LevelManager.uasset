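; Level manager that runs enemy spawning, the match countdown and the score goal.
; On BeginPlay it gathers all BP_Enemy_SpawnPoint actors, and a looping timer tells a random one to spawn an enemy.
; Tick uses a one-second Delay to count down minutes and seconds, and also checks the score fed by AddTargetPoints.
; Time running out or reaching the required score shows the same game-over widget and pauses, a prototype placeholder for winning.
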(event `self.ReceiveBeginPlay`
  ;[1 1 1] Spawn enemy at random set point
  (bind _outactors (`GameplayStatics.GetAllActorsOfClass` "/Game/Blueprints/WaveManagement/BP_Enemy_SpawnPoint.BP_Enemy_SpawnPoint_C"))
  ;;[1 1 1] Time til next enemy spawn
  (set `self.Spawner list` _outactors)
  (`KismetSystemLibrary.K2_SetTimerDelegate` (delegate `ActivateSpawner`) (`self.Time between next enemy spawn`) true))

(event `ActivateSpawner`
  (bind _spawner_list (`self.Spawner list`))
  ;[1 1 1] Spawn enemy at random set point
  ;;[1 1 1] Get random Spawn point
  (`/Game/Blueprints/WaveManagement/BP_Enemy_SpawnPoint.SpawnEnemy` (`|GetArrayItem` _spawner_list (`KismetMathLibrary.RandomIntegerInRange` 0 (- (`KismetArrayLibrary.Array_Length` _spawner_list) 1)))))

(event `self.ReceiveTick`
  (params (DeltaSeconds :type "Float (single-precision)"))
  (`|ExecutionSequence`
    (:`then_0`
      ;[1 1 1] Timer counting down
      (`KismetSystemLibrary.Delay` 1.0)
      (if (== (`self.Seconds`) 0)
        (if (== (`self.Minutes`) 0)
          ;;[1 1 1] Put up game over widget if timer reach to 00:00
          (bind _returnvalue (`|CreateWidget` "/Game/Widget/UI_GameOver.UI_GameOver_C"))
          (`UserWidget.AddToViewport` _returnvalue 0)
          (set `PlayerController.bShowMouseCursor` true (`GameplayStatics.GetPlayerController` 0))
          (`GameplayStatics.SetGamePaused` true)
          (else
            (set `self.Seconds` 59)
            (set `self.Minutes` (- (`self.Minutes`) 1))))
        (else
          (set `self.Seconds` (- (`self.Seconds`) 1)))))
    (:`then_1`
      ;[1 1 1] Win condition meet
      (if (>= (`self.Score`) (`self.RequiredScore`))
        ;[1 1 1] Temporary for prototype
        (`/Engine/EditorBlueprintResources/StandardMacros.DoOnce` false
          (:`Completed`
            (bind _returnvalue_2 (`|CreateWidget` "/Game/Widget/UI_GameOver.UI_GameOver_C"))
            (`UserWidget.AddToViewport` _returnvalue_2 0)
            (set `PlayerController.bShowMouseCursor` true (`GameplayStatics.GetPlayerController` 0))
            (`GameplayStatics.SetGamePaused` true)))))))

(event `AddTargetPoints`
  (params (TargetScore :type Integer))
  ;[1 1 1] Set Score
  (set `self.Score` (+ TargetScore (`self.Score`))))

(fn `UserConstructionScript`)