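; Ranged fairy mech enemy AI Blueprint that fires a bullet at the player once it finishes landing at distance.
; FinishedLandingAtDistance turns Arrow1 toward the first player pawn, then spawns BP_EnemyBullet at the arrow's transform and prints a debug string.
; BeginPlay and construction only call the parent, so other behavior is left to the parent class.
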(event `self.ReceiveBeginPlay`
  (`parent.ReceiveBeginPlay`))

(fn `FinishedLandingAtDistance`
  (bind _arrow1 (`self.Arrow1`))
  (`KismetSystemLibrary.PrintString` "pew pew")
  (`SceneComponent.K2_SetWorldRotation` _arrow1 (`KismetMathLibrary.FindLookAtRotation` (`SceneComponent.K2_GetComponentLocation` _arrow1) (`SceneComponent.K2_GetComponentLocation` (`Actor.RootComponent` (`GameplayStatics.GetPlayerPawn` 0)))) false false)
  (`|SpawnActorFromClass` "/Game/Blueprints/Projectiles/BP_EnemyBullet.BP_EnemyBullet_C" (`SceneComponent.K2_GetComponentToWorld` (`self.Arrow1`)) "Undefined" "OverrideRootScale" null null))

(fn `UserConstructionScript`
  (`parent.UserConstructionScript`))