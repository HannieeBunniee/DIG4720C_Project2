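; BP_AIEnemy_DropShip_Manta is a water-enemy drop ship that deploys other AI enemies when it finishes landing.
; BeginPlay runs the parent logic, then sets its maximum and current health.
; FinishedLandingAtDistance prints a debug message and spawns one AI pawn of a random class from SpawnerList at the Arrow1 component's location.
; The file contains no movement or landing logic of its own.
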(event `self.ReceiveBeginPlay`
  (`parent.ReceiveBeginPlay`)
  (set `self.EnemyMaxHealth` 1000.0)
  (set `self.EnemyCurrentHealth` 1000.0))

(fn `FinishedLandingAtDistance`
  (locals (`Spawner List` :type "Array of Pawn Class Reference"))
  (`KismetSystemLibrary.PrintString` "spawning enemy")
  (`AIBlueprintHelperLibrary.SpawnAIFromClass` (`KismetArrayLibrary.Array_Random` (`local.Spawner List`)) null (`SceneComponent.K2_GetComponentLocation` (`self.Arrow1`)) (struct) false null))

(fn `UserConstructionScript`
  (`parent.UserConstructionScript`))