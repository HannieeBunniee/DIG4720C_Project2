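; Zombie variant of the AI enemy drop ship, which delivers zombie enemies when it lands.
; On BeginPlay it runs the parent logic, then overrides its current and maximum health with fixed values.
; Its FinishedLandingAtDistance function spawns an AI pawn of a random class from SpawnerList at the Arrow1 component's world location.
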(event `self.ReceiveBeginPlay`
  (`parent.ReceiveBeginPlay`)
  (set `self.EnemyCurrentHealth` 500.0)
  (set `self.EnemyMaxHealth` 500.0))

(fn `FinishedLandingAtDistance`
  (locals (`Spawner List` :type "Array of Pawn Class Reference"))
  (`AIBlueprintHelperLibrary.SpawnAIFromClass` (`KismetArrayLibrary.Array_Random` (`local.Spawner List`)) null (`SceneComponent.K2_GetComponentLocation` (`self.Arrow1`)) (struct) false null))

(fn `UserConstructionScript`
  (`parent.UserConstructionScript`))