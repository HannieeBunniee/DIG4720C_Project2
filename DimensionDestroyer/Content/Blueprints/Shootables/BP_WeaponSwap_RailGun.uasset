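; BP_WeaponSwap_RailGun is a shootable weapon-swap pickup that gives the player the rail gun.
; On BeginPlay it sets its swap name to RailGun before running the parent's setup.
; Its SetPlayerWeapon event destroys the character's current gun child actor and sets the Gun component's child actor class to BP_Gun_Rail.
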(event `self.ReceiveBeginPlay`
  (set `self.WeaponSwapName` "RailGun")
  (`parent.ReceiveBeginPlay`))

(event `self.SetPlayerWeapon`
  (`self.K2_DestroyActor` (`ChildActorComponent.ChildActor` (`/Game/Blueprints/Player/BP_PlayerCharacter.Gun` (`self.Character`))))
  (`ChildActorComponent.SetChildActorClass` (`/Game/Blueprints/Player/BP_PlayerCharacter.Gun` (`self.Character`)) "/Game/Blueprints/Weapons/BP_Gun_Rail.BP_Gun_Rail_C"))

(fn `UserConstructionScript`
  (`parent.UserConstructionScript`))