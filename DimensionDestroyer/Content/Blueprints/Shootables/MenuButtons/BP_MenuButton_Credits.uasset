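; Shootable Credits button that switches the menu to the credits state when it takes damage.
; It runs the parent damage handling, waits briefly, then destroys all Play and Quit button actors.
; It then hides its text render, spawns a CreditsBack button at a fixed world transform and destroys itself.
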(event `self.ReceiveAnyDamage`
  (params (Damage :type "Float (single-precision)") (DamageType :type "DamageType Object Reference") (InstigatedBy :type "Controller Object Reference") (DamageCauser :type "Actor Object Reference"))
  (`parent.ReceiveAnyDamage` Damage null null null)
  (`KismetSystemLibrary.Delay` 0.2)
  (`|ExecutionSequence`
    (:`then_0`
      (bind _outactors (`GameplayStatics.GetAllActorsOfClass` "/Game/Blueprints/Shootables/MenuButtons/BP_MenuButton_Play.BP_MenuButton_Play_C"))
      (`self.K2_DestroyActor` _outactors))
    (:`then_1`
      (bind _outactors_2 (`GameplayStatics.GetAllActorsOfClass` "/Game/Blueprints/Shootables/MenuButtons/BP_MenuButton_Quit.BP_MenuButton_Quit_C"))
      (`self.K2_DestroyActor` _outactors_2))
    (:`then_2`
      (`SceneComponent.SetVisibility` (`self.TextRender`) false false)
      (`|SpawnActorFromClass` "/Game/Blueprints/Shootables/MenuButtons/BP_MenuButton_CreditsBack.BP_MenuButton_CreditsBack_C" (`KismetMathLibrary.MakeTransform` (2500.0 0.0 600.0) (struct :`Yaw` 180.0)) "Undefined" "OverrideRootScale" null null))
    (:`then_3`
      (`self.K2_DestroyActor`))))

(fn `UserConstructionScript`
  (`parent.UserConstructionScript`))