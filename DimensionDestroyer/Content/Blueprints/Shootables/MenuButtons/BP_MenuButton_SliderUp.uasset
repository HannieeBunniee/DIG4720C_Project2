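; BP_MenuButton_SliderUp is a shootable menu button that nudges the slider of its parent BP_Slider actor when it takes damage.
; On damage it runs the inherited handler, waits briefly, then sets its text color.
; It then casts its parent actor to BP_Slider and steps SliderMesh along negative relative Y, clamped to a fixed travel range.
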(event `self.ReceiveAnyDamage`
  (params (Damage :type "Float (single-precision)") (DamageType :type "DamageType Object Reference") (InstigatedBy :type "Controller Object Reference") (DamageCauser :type "Actor Object Reference"))
  (`parent.ReceiveAnyDamage` Damage null null null)
  (`KismetSystemLibrary.Delay` 0.2)
  (`TextRenderComponent.SetTextRenderColor` (`self.TextRender`) (`self.Value`))
  (bind _asbp_slider (cast `/Game/Blueprints/Shootables/MenuButtons/BP_Slider` (`self.GetParentActor`)))
  (bind _slidermesh (`/Game/Blueprints/Shootables/MenuButtons/BP_Slider.SliderMesh` _asbp_slider))
  (bind (_relativelocation_x _relativelocation_y _relativelocation_z) (`KismetMathLibrary.BreakVector` (`SceneComponent.RelativeLocation` _slidermesh)))
  (`SceneComponent.K2_SetRelativeLocation` _slidermesh (`KismetMathLibrary.MakeVector` _relativelocation_x (`KismetMathLibrary.FClamp` (- _relativelocation_y 100.0) -500.0 500.0) _relativelocation_z) false false))

(fn `UserConstructionScript`
  (`parent.UserConstructionScript`))