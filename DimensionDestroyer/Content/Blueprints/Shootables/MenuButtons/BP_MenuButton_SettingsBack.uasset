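; Shootable menu button that backs out of the settings screen to the main menu when it takes damage.
; It runs the parent damage handling, waits a second, then clears the slider actors found in the level.
; It rebuilds the main menu by spawning Play, Quit and Settings buttons at hardcoded transforms, then destroys itself.
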(event `self.ReceiveAnyDamage`
  (params (Damage :type "Float (single-precision)") (DamageType :type "DamageType Object Reference") (InstigatedBy :type "Controller Object Reference") (DamageCauser :type "Actor Object Reference"))
  (`parent.ReceiveAnyDamage` Damage null null null)
  (`KismetSystemLibrary.Delay` 1.0)
  (`|ExecutionSequence`
    (:`then_0`
      (bind _outactors (`GameplayStatics.GetAllActorsOfClass` "/Game/Blueprints/Shootables/MenuButtons/BP_Slider.BP_Slider_C"))
      (`self.K2_DestroyActor` _outactors))
    (:`then_1`
      (`|SpawnActorFromClass` "/Game/Blueprints/Shootables/MenuButtons/BP_MenuButton_Play.BP_MenuButton_Play_C" (`KismetMathLibrary.MakeTransform` (2500.0 -1000.0 1400.0) (struct :`Yaw` 180.0) (1.0 1.0 1.0)) "Undefined" "OverrideRootScale" null null)
      (`|SpawnActorFromClass` "/Game/Blueprints/Shootables/MenuButtons/BP_MenuButton_Quit.BP_MenuButton_Quit_C" (`KismetMathLibrary.MakeTransform` (2500.0 1000.0 1400.0) (struct :`Yaw` 180.0)) "Undefined" "OverrideRootScale" null null))
    (:`then_2`
      (`|SpawnActorFromClass` "/Game/Blueprints/Shootables/MenuButtons/BP_MenuButton_Settings.BP_MenuButton_Settings_C" (`KismetMathLibrary.MakeTransform` (2200.0 0.0 600.0) (struct :`Yaw` 180.0)) "Undefined" "OverrideRootScale" null null)
      (`self.K2_DestroyActor`))))

(fn `UserConstructionScript`
  (`parent.UserConstructionScript`))