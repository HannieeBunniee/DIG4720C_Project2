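; BP_MenuButton_Play is a shootable menu button that opens a level when it receives damage.
; On AnyDamage it runs the parent handler, then adds a UI_LoadingScreen widget to the viewport.
; It disables player input and stops the gun firing so shooting cannot continue during loading.
; The loading screen fades in, and after a short delay the level named by LevelName opens.
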(event `self.ReceiveAnyDamage`
  (params (Damage :type "Float (single-precision)") (DamageType :type "DamageType Object Reference") (InstigatedBy :type "Controller Object Reference") (DamageCauser :type "Actor Object Reference"))
  (`parent.ReceiveAnyDamage` Damage null null null)
  ;[1 1 1] Loading screen
  (bind _returnvalue (`|CreateWidget` "/Game/Widget/UI_LoadingScreen.UI_LoadingScreen_C"))
  (`UserWidget.AddToViewport` _returnvalue 0)
  ;;[1 1 1] Stop player from able to shoot while in loading screen
  (bind _returnvalue_2 (`GameplayStatics.GetActorOfClass` "/Game/Blueprints/Player/BP_PlayerCharacter.BP_PlayerCharacter_C"))
  (`self.DisableInput` _returnvalue_2 (`GameplayStatics.GetPlayerController` 0))
  ;;[1 1 1] Stop gun from keep shooting
  (bind _returnvalue_3 (`GameplayStatics.GetActorOfClass` "/Game/Blueprints/Weapons/BP_Gun_Master.BP_Gun_Master_C"))
  (`/Game/Blueprints/Weapons/BP_Gun_Master.StopShooting` _returnvalue_3)
  (`/Game/Widget/UI_LoadingScreen.FadeIn` _returnvalue)
  (`KismetSystemLibrary.Delay` 1.0)
  (`GameplayStatics.OpenLevel` (`self.Level Name`)))

(fn `UserConstructionScript`
  (`parent.UserConstructionScript`))