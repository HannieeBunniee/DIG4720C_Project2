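; BP_Gun_Gatling is a twin-barrel Gatling gun weapon that extends a parent gun Blueprint with rapid alternating fire.
; BeginPlay gives it an effectively bottomless clip and sets its base damage.
; StartShooting runs looping FireBulletLeft and FireBulletRight timers at FireRate, delaying the right by half an interval so shots alternate.
; StopShooting clears both timers; the fire functions are not defined in these graphs.
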(event `self.ReceiveBeginPlay`
  (`parent.ReceiveBeginPlay`)
  (set `self.AmmoCurrent` 10000000)
  (set `self.AmmoClipMax` 10000000)
  (set `self.BaseDamage` 20.0))

(event `self.StartShooting`
  (`parent.StartShooting`)
  (bind _returnvalue (`KismetSystemLibrary.K2_SetTimer` null "FireBulletLeft" (`self.FireRate`) true))
  (set `self.GunTimerLeft` _returnvalue)
  (bind _returnvalue_2 (`KismetSystemLibrary.K2_SetTimer` null "FireBulletRight" (`self.FireRate`) true (/ (`self.FireRate`) 2.0)))
  (set `self.GunTimerRight` _returnvalue_2))

(event `self.StopShooting`
  (`parent.StopShooting`)
  (`KismetSystemLibrary.K2_ClearAndInvalidateTimerHandle` (`self.GunTimerLeft`))
  (`KismetSystemLibrary.K2_ClearAndInvalidateTimerHandle` (`self.GunTimerRight`)))

(fn `UserConstructionScript`
  (`parent.UserConstructionScript`))