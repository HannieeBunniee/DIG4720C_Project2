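; Twin-barrel rocket launcher weapon for the player that fires rockets from left and right muzzle arrows while shooting is held.
; StartShooting fires both barrels at once and starts looping timers at FireRate, gated by a short CanShoot cooldown; StopShooting clears both timers.
; Each shot traces from the camera and aims a spawned BP_Projectile_Rocket at the hit or maximum-range point.
; Only the left barrel plays the sound and camera shake.
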(event `self.ReceiveBeginPlay`
  (`parent.ReceiveBeginPlay`))

(event `EnableFire`
  (set `self.CanShoot` true))

(event `self.StartShooting`
  (`parent.StartShooting`)
  (if (`self.CanShoot`)
    (`KismetSystemLibrary.K2_SetTimerDelegate` (delegate `EnableFire`) 0.4)
    (set `self.CanShoot` false)
    (`self.FireRocketLeft`)
    (bind _returnvalue (`KismetSystemLibrary.K2_SetTimer` null "FireRocketLeft" (`self.FireRate`) true))
    (set `self.GunTimerLeft` _returnvalue)
    (`self.FireRocketRight`)
    (bind _returnvalue_2 (`KismetSystemLibrary.K2_SetTimer` null "FireRocketRight" (`self.FireRate`) true))
    (set `self.GunTimerRight` _returnvalue_2)))

(event `self.StopShooting`
  (`parent.StopShooting`)
  (`KismetSystemLibrary.K2_ClearAndInvalidateTimerHandle` (`self.GunTimerLeft`))
  (`KismetSystemLibrary.K2_ClearAndInvalidateTimerHandle` (`self.GunTimerRight`)))

(fn `FireRocketLeft`
  (locals (BulletDistance :type "Float (double-precision)" :default 10000.0))
  (bind _returnvalue (`SceneComponent.K2_GetComponentLocation` (`self.ArrowLeft`)))
  (bind _asbp_player_character (cast `/Game/Blueprints/Player/BP_PlayerCharacter` (`GameplayStatics.GetPlayerCharacter` 0)))
  (`|ExecutionSequence`
    (:`then_0`
      (bind _camera (`/Game/Blueprints/Player/BP_PlayerCharacter.Camera` _asbp_player_character))
      (bind _returnvalue_2 (`SceneComponent.K2_GetComponentLocation` _camera))
      (bind _returnvalue_3 (+ _returnvalue_2 (* (`KismetMathLibrary.GetForwardVector` (`SceneComponent.K2_GetComponentRotation` _camera)) (`local.BulletDistance`))))
      ;[1 1 1] Gets cursor location in world.
      (bind (_outhit _returnvalue_4) (`KismetSystemLibrary.LineTraceSingle` :`Start` _returnvalue_2 :`End` _returnvalue_3 :`TraceChannel` "TraceTypeQuery1" :`TraceColor` (struct :`G` 1.0 :`B` 1.0 :`A` 1.0) :`DrawTime` 1.0))
      (if _returnvalue_4
        (set `self.BulletImpactPoint_0` (`.ImpactPoint` (`GameplayStatics.BreakHitResult` _outhit)))
        (else
          (set `self.BulletImpactPoint_0` _returnvalue_3))))
    (:`then_1`
      (`|SpawnActorFromClass` "/Game/Blueprints/Projectiles/BP_Projectile_Rocket.BP_Projectile_Rocket_C" (`KismetMathLibrary.MakeTransform` _returnvalue (`KismetMathLibrary.FindLookAtRotation` _returnvalue (`self.BulletImpactPoint_0`))) "AdjustIfPossibleButAlwaysSpawn" "OverrideRootScale" null null)
      (`GameplayStatics.SpawnSound2D` "/Game/Sound/SFX/Underwater_Explosion.Underwater_Explosion" 0.3 3.0 0.0 null)
      (`GameplayStatics.PlayWorldCameraShake` "/Game/Blueprints/CameraShake.CameraShake_C" (0.0 0.0 0.0) 0.0 10000.0))))

(fn `FireRocketRight`
  (locals (BulletDistance :type "Float (double-precision)" :default 10000.0))
  (bind _returnvalue (`SceneComponent.K2_GetComponentLocation` (`self.ArrowRight`)))
  (bind _asbp_player_character (cast `/Game/Blueprints/Player/BP_PlayerCharacter` (`GameplayStatics.GetPlayerCharacter` 0)))
  (`|ExecutionSequence`
    (:`then_0`
      (bind _camera (`/Game/Blueprints/Player/BP_PlayerCharacter.Camera` _asbp_player_character))
      (bind _returnvalue_2 (`SceneComponent.K2_GetComponentLocation` _camera))
      (bind _returnvalue_3 (+ _returnvalue_2 (* (`KismetMathLibrary.GetForwardVector` (`SceneComponent.K2_GetComponentRotation` _camera)) (`local.BulletDistance`))))
      ;[1 1 1] Gets cursor location in world.
      (bind (_outhit _returnvalue_4) (`KismetSystemLibrary.LineTraceSingle` :`Start` _returnvalue_2 :`End` _returnvalue_3 :`TraceChannel` "TraceTypeQuery1" :`TraceColor` (struct :`G` 1.0 :`B` 1.0 :`A` 1.0) :`DrawTime` 1.0))
      (if _returnvalue_4
        (set `self.BulletImpactPoint_0` (`.ImpactPoint` (`GameplayStatics.BreakHitResult` _outhit)))
        (else
          (set `self.BulletImpactPoint_0` _returnvalue_3))))
    (:`then_1`
      (`|SpawnActorFromClass` "/Game/Blueprints/Projectiles/BP_Projectile_Rocket.BP_Projectile_Rocket_C" (`KismetMathLibrary.MakeTransform` _returnvalue (`KismetMathLibrary.FindLookAtRotation` _returnvalue (`self.BulletImpactPoint_0`))) "AdjustIfPossibleButAlwaysSpawn" "OverrideRootScale" null null))))

(fn `UserConstructionScript`
  (`parent.UserConstructionScript`))