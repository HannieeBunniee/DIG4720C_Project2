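; BP_Gun_Master is a gun base for the player character, with left and right barrels, clip ammo and a firing flag.
; Fire functions trace from the camera for an aim point, then from the barrel arrows toward it, damaging actors other than the player.
; Lasers multi-trace from both barrels for one ammo; bullets single-trace per side, spending ammo and spawning a Niagara burst only on valid hits.
; Nothing here calls the fire functions.
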(event `self.ReceiveBeginPlay`
  (bind _asbp_player_character (cast `/Game/Blueprints/Player/BP_PlayerCharacter` (`GameplayStatics.GetPlayerCharacter` 0)))
  (set `self.Character` _asbp_player_character))

(event `StartShooting`
  (set `self.IsFiring` true))

(event `StopShooting`
  (set `self.IsFiring` false))

(fn `FireBulletLeft`
  (bind _camera (`/Game/Blueprints/Player/BP_PlayerCharacter.Camera` (`self.Character`)))
  (bind _returnvalue (`SceneComponent.K2_GetComponentLocation` _camera))
  (bind _returnvalue_2 (+ _returnvalue (* (`KismetMathLibrary.GetForwardVector` (`SceneComponent.K2_GetComponentRotation` _camera)) (`self.BulletDistance`))))
  (if (`self.HasAmmoInClip`)
    (`|ExecutionSequence`
      (:`then_0`
        ;[1 1 1] Gets cursor location in world.
        (bind (_outhit _returnvalue_3) (`KismetSystemLibrary.LineTraceSingle` :`Start` _returnvalue :`End` _returnvalue_2 :`TraceChannel` "TraceTypeQuery1" :`TraceColor` (struct :`G` 1.0 :`B` 1.0 :`A` 1.0) :`DrawTime` 1.0))
        (if _returnvalue_3
          (set `self.BulletImpactPoint` (`.ImpactPoint` (`GameplayStatics.BreakHitResult` _outhit)))
          (else
            (set `self.BulletImpactPoint` _returnvalue_2))))
      (:`then_1`
        ;[1 1 1] Fires bullets from left gun. Bullets will travel from barrel to cursor location in the world.
        (bind (_outhit_2 _returnvalue_4) (`KismetSystemLibrary.LineTraceSingle` :`Start` (`SceneComponent.K2_GetComponentLocation` (`self.ArrowLeft`)) :`End` (+ (`self.BulletImpactPoint`) (`SceneComponent.GetForwardVector` (`self.ArrowLeft`))) :`TraceChannel` "TraceTypeQuery1" :`DrawTime` 1.0))
        (if _returnvalue_4
          (bind (_bblockinghit _binitialoverlap _time _distance _location _impactpoint _normal _impactnormal _physmat _hitactor) (`GameplayStatics.BreakHitResult` _outhit_2))
          (if (!= _hitactor (`self.Character`))
            (`GameplayStatics.ApplyDamage` _hitactor (`self.BaseDamage`))
            (bind _result (`/Engine/EditorBlueprintResources/StandardMacros.DecrementInt` (`self.AmmoCurrent`))
              (:`  `
                (set `self.AmmoCurrent` (`KismetMathLibrary.Clamp` _result 0 (`self.AmmoClipMax`)))
                (`NiagaraFunctionLibrary.SpawnSystemAtLocation` "/Game/VFX/Burst/NS_Burst.NS_Burst" (`self.BulletImpactPoint`))))))))))

(fn `FireBulletRight`
  (bind _camera (`/Game/Blueprints/Player/BP_PlayerCharacter.Camera` (`self.Character`)))
  (bind _returnvalue (`SceneComponent.K2_GetComponentLocation` _camera))
  (bind _returnvalue_2 (+ _returnvalue (* (`KismetMathLibrary.GetForwardVector` (`SceneComponent.K2_GetComponentRotation` _camera)) (`self.BulletDistance`))))
  (if (`self.HasAmmoInClip`)
    (`|ExecutionSequence`
      (:`then_0`
        ;[1 1 1] Gets cursor location in world.
        (bind (_outhit _returnvalue_3) (`KismetSystemLibrary.LineTraceSingle` :`Start` _returnvalue :`End` _returnvalue_2 :`TraceChannel` "TraceTypeQuery1" :`TraceColor` (struct :`G` 1.0 :`B` 1.0 :`A` 1.0) :`DrawTime` 1.0))
        (if _returnvalue_3
          (set `self.BulletImpactPoint` (`.ImpactPoint` (`GameplayStatics.BreakHitResult` _outhit)))
          (else
            (set `self.BulletImpactPoint` _returnvalue_2))))
      (:`then_1`
        ;[1 1 1] Fires bullets from right gun. Bullets will travel from barrel to cursor location in the world.
        (bind (_outhit_2 _returnvalue_4) (`KismetSystemLibrary.LineTraceSingle` :`Start` (`SceneComponent.K2_GetComponentLocation` (`self.ArrowRight`)) :`End` (+ (`self.BulletImpactPoint`) (`SceneComponent.GetForwardVector` (`self.ArrowRight`))) :`TraceChannel` "TraceTypeQuery1" :`DrawTime` 1.0))
        (if _returnvalue_4
          (bind (_bblockinghit _binitialoverlap _time _distance _location _impactpoint _normal _impactnormal _physmat _hitactor) (`GameplayStatics.BreakHitResult` _outhit_2))
          (if (!= _hitactor (`self.Character`))
            (`GameplayStatics.ApplyDamage` _hitactor (`self.BaseDamage`))
            (bind _result (`/Engine/EditorBlueprintResources/StandardMacros.DecrementInt` (`self.AmmoCurrent`))
              (:`  `
                (set `self.AmmoCurrent` (`KismetMathLibrary.Clamp` _result 0 (`self.AmmoClipMax`)))
                (`NiagaraFunctionLibrary.SpawnSystemAtLocation` "/Game/VFX/Burst/NS_Burst.NS_Burst" (`self.BulletImpactPoint`))))))))))

(fn `FireLasers`
  (bind _camera (`/Game/Blueprints/Player/BP_PlayerCharacter.Camera` (`self.Character`)))
  (bind _returnvalue (`SceneComponent.K2_GetComponentLocation` _camera))
  (bind _returnvalue_2 (+ _returnvalue (* (`KismetMathLibrary.GetForwardVector` (`SceneComponent.K2_GetComponentRotation` _camera)) (`self.BulletDistance`))))
  (if (`self.HasAmmoInClip`)
    (`|ExecutionSequence`
      (:`then_0`
        ;[1 1 1] Gets cursor location in world.
        (bind (_outhit _returnvalue_3) (`KismetSystemLibrary.LineTraceSingle` :`Start` _returnvalue :`End` _returnvalue_2 :`TraceChannel` "TraceTypeQuery1" :`TraceColor` (struct :`G` 1.0 :`B` 1.0 :`A` 1.0) :`DrawTime` 1.0))
        (if _returnvalue_3
          (set `self.BulletImpactPoint` (`.ImpactPoint` (`GameplayStatics.BreakHitResult` _outhit)))
          (else
            (set `self.BulletImpactPoint` _returnvalue_2))))
      (:`then_1`
        ;[1 1 1] Fires Laser from right gun. Bullets will travel from barrel to cursor location in the world.
        (bind _outhits (`KismetSystemLibrary.LineTraceMulti` (`SceneComponent.K2_GetComponentLocation` (`self.ArrowRight`)) (+ (`self.BulletImpactPoint`) (`SceneComponent.GetForwardVector` (`self.ArrowRight`))) "TraceTypeQuery1"))
        (for _array_element _outhits
          (bind (_bblockinghit _binitialoverlap _time _distance _location _impactpoint _normal _impactnormal _physmat _hitactor) (`GameplayStatics.BreakHitResult` _array_element))
          (if (!= _hitactor (`self.Character`))
            (`GameplayStatics.ApplyDamage` _hitactor (`self.BaseDamage`))))
        (bind _result (`/Engine/EditorBlueprintResources/StandardMacros.DecrementInt` (`self.AmmoCurrent`))
          (:`  `
            (set `self.AmmoCurrent` (`KismetMathLibrary.Clamp` _result 0 (`self.AmmoClipMax`)))
            (`NiagaraFunctionLibrary.SpawnSystemAtLocation` "/Game/VFX/Burst/NS_Burst.NS_Burst" (`self.BulletImpactPoint`)))))
      (:`then_2`
        ;[1 1 1] Fires Laser from right gun. Bullets will travel from barrel to cursor location in the world.
        (bind _outhits_2 (`KismetSystemLibrary.LineTraceMulti` (`SceneComponent.K2_GetComponentLocation` (`self.ArrowLeft`)) (+ (`self.BulletImpactPoint`) (`SceneComponent.GetForwardVector` (`self.ArrowLeft`))) "TraceTypeQuery1"))
        (for _array_element_2 _outhits_2
          (bind (_bblockinghit_2 _binitialoverlap_2 _time_2 _distance_2 _location_2 _impactpoint_2 _normal_2 _impactnormal_2 _physmat_2 _hitactor_2) (`GameplayStatics.BreakHitResult` _array_element_2))
          (if (!= _hitactor_2 (`self.Character`))
            (`GameplayStatics.ApplyDamage` _hitactor_2 (`self.BaseDamage`))))))))

(fn `HasAmmoInClip`
  (returns (ReturnValue :type Boolean))
  (return (> (`self.AmmoCurrent`) 0)))

(fn `UserConstructionScript`)