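; Rail gun weapon that extends a parent gun with a charge-up laser shot and a charge bar HUD widget.
; Holding fire plays a timeline scaled by ChargeTime to build CurrentCharge, firing on release above a minimum or automatically at full charge.
; Damage scales with charge by temporarily modifying BaseDamage around the parent's FireLasers.
; Stopping reverses the timeline, and a new charge requires low remaining charge and available ammo.
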(event `self.ReceiveBeginPlay`
  (`parent.ReceiveBeginPlay`)
  (set `self.AmmoCurrent` 1000)
  (bind _returnvalue (`|CreateWidget` "/Game/Widget/UI_ChargeBarHUD.UI_ChargeBarHUD_C"))
  (bind _output_get (set `self.ChargeUI` _returnvalue))
  (`UserWidget.AddToViewport` _output_get 0))

(event `self.StartShooting`
  (`parent.StartShooting`)
  (if (`self.CanCharge`)
    (set `self.IsCharging` true)
    (`TimelineComponent.SetPlayRate` (`self.T_ChargeWeapon`) (/ 1.0 (`self.ChargeTime`)))
    (bind (_direction _weaponcharge) (`Timeline|T_ChargeWeapon` :!label _label)
      (:`Update`
        (bind _output_get (set `self.CurrentCharge` (`KismetMathLibrary.FClamp` _weaponcharge)))
        (if (>= _output_get 1.0)
          (`self.StopShooting`))))))

(event `self.StopShooting`
  (`parent.StopShooting`)
  (if (`self.CanShoot`)
    (`self.FireLasers`))
  (set `self.IsCharging` false)
  (`TimelineComponent.SetPlayRate` (`self.T_ChargeWeapon`) 1.0)
  (goto _label :!via `Reverse`))

(event `self.FireLasers`
  (set `self.BaseDamage` (* (`self.BaseDamage`) (`self.CurrentCharge`)))
  (`parent.FireLasers`)
  (set `self.BaseDamage` 50.0))

(fn `CanCharge`
  (returns (ReturnValue :type Boolean))
  (return (and (not (`self.IsCharging`)) (<= (`self.CurrentCharge`) 0.2) (> (`self.AmmoCurrent`) 0))))

(fn `CanShoot`
  (returns (ReturnValue :type Boolean))
  (return (and (`self.IsCharging`) (>= (`self.CurrentCharge`) 0.2))))

(fn `UserConstructionScript`
  (`parent.UserConstructionScript`))