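; Test wave manager that runs numbered enemy waves, each preceded by a short printed countdown.
; On BeginPlay it sorts level spawn points into ground, air and turret lists.
; Each wave reads its data table row by wave number and spawns enemies at random points of the matching type.
; It then polls enemy validity every second to decide when to advance, with boss or level-end handling still a placeholder.
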(event `self.ReceiveBeginPlay`
  ;[1 1 1] Sort enemy spawner reference
  (bind _outactors (`GameplayStatics.GetAllActorsOfClass` "/Game/Blueprints/WaveSpawn/Test/BP_WaveSpawnPoint.BP_WaveSpawnPoint_C"))
  (bind _output_get (set `self.EnemySpawnPoints` _outactors))
  (for _array_element _output_get
    (switch `/Game/Blueprints/WaveSpawn/Test/E_EnemyType` (`/Game/Blueprints/WaveSpawn/Test/BP_WaveSpawnPoint.SpawnerType` _array_element)
      (:`NewEnumerator0`
        (`KismetArrayLibrary.Array_Add` (`self.E_Ground`) _array_element))
      (:`NewEnumerator1`
        (`KismetArrayLibrary.Array_Add` (`self.E_Air`) _array_element))
      (:`NewEnumerator2`
        (`KismetArrayLibrary.Array_Add` (`self.E_Turret`) _array_element))))
  (`self.CountDown`))

(event `CountDown`
  ;[1 1 1] Countdown
  (bind _returnvalue (`KismetSystemLibrary.K2_SetTimerDelegate` (delegate `Count`) 1.0 true))
  (set `self.Countdown_Time` 3))

(event `Count`
  ;[1 1 1] Countdown
  (`KismetSystemLibrary.PrintString` (`KismetStringLibrary.Conv_IntToString` (`self.Countdown_Time`)))
  (if (== (`self.Countdown_Time`) 0)
    (`KismetSystemLibrary.K2_ClearAndInvalidateTimerHandle` (stale `CountDown` _returnvalue))
    (`self.Begin Wave`)
    (else
      (`/Engine/EditorBlueprintResources/StandardMacros.DecrementInt` (`self.Countdown_Time`)))))

(event `Begin Wave`
  ;[1 1 1] Spawn Enemies for wave
  (`KismetSystemLibrary.PrintString` "Wave Begin")
  (bind _returnvalue (`|GetDataTableRow` (`self.EnemyDataTable`) (`KismetStringLibrary.Conv_StringToName` (`KismetStringLibrary.Conv_IntToString` (`self.WaveNumber`))))
    (:`then`
      (for _array_element (`.EnemyInfos_3_9F8711CE433AC6C37BC74DAD04AFFCA8` (break `/Game/Blueprints/WaveSpawn/Test/WaveInfos` _returnvalue))
        (`self.SpawnEnemies` _array_element))
      (`self.Start Checking if enemies are dead`))
    (:`RowNotFound`
      (`KismetSystemLibrary.PrintString` "Couldnt find row for wave data"))))

(event `Start Checking if enemies are dead`
  ;[1 1 1] Check if enemies are dead and start new wave
  (bind _aredead_1 (`self.CheckIfAllEnemiesAreDead` :!label _label))
  (if _aredead_1
    (`KismetSystemLibrary.PrintString` "You killed all enemies! YEYYY" true true (struct :`G` 1.0 :`B` 0.057168 :`A` 1.0))
    (`/Engine/EditorBlueprintResources/StandardMacros.IncrementInt` (`self.WaveNumber`)
      (:`  `
        (if true
          (`self.CountDown`))))
    (else
      (`KismetSystemLibrary.Delay` 1.0)
      (goto _label))))

(fn `CheckIfAllEnemiesAreDead`
  (returns (`AreDead?1` :type Boolean))
  (locals (`AreDead?` :type Boolean))
  (set `local.AreDead?` true)
  (for _array_element (`self.CurrentEnemies`)
    (`/Engine/EditorBlueprintResources/StandardMacros.IsValid` _array_element
      (:`Is Valid`
        (set `local.AreDead?` false))
      (:`Is Not Valid`
        (return (`local.AreDead?`))))))

(fn `SpawnEnemies`
  (params (EnemyInfo :type "/Game/Blueprints/WaveSpawn/Test/EnemyInfo Structure (by ref)"))
  (locals (CurrentSpawnPoint :type "Array of /Game/Blueprints/WaveSpawn/Test/BP_WaveSpawnPoint Object Reference") (EnemyInfoRef :type "/Game/Blueprints/WaveSpawn/Test/EnemyInfo Structure"))
  (bind _enemyinforef_enemyclass (break `/Game/Blueprints/WaveSpawn/Test/EnemyInfo` (`local.EnemyInfoRef`)))
  (bind (_enemyinforef_enemyclass_2 _enemyinforef_enemynumber) (break `/Game/Blueprints/WaveSpawn/Test/EnemyInfo` (`local.EnemyInfoRef`)))
  (bind _currentspawnpoint (`local.CurrentSpawnPoint`))
  ;[1 1 1] Spawn Enemies function
  (set `local.EnemyInfoRef` EnemyInfo)
  (set `local.CurrentSpawnPoint` (select `/Game/Blueprints/WaveSpawn/Test/E_EnemyType` (`.EnemyType_10_7E8DDE6D412ABE9D156BC2A21B5CD02B` (break `/Game/Blueprints/WaveSpawn/Test/EnemyInfo` EnemyInfo)) :`NewEnumerator0` (`self.E_Ground`) :`NewEnumerator1` (`self.E_Air`) :`NewEnumerator2` (`self.E_Turret`)))
  (for _ (range 1 (+ _enemyinforef_enemynumber 1))
    (bind _returnvalue (`|SpawnActorFromClass` _enemyinforef_enemyclass (`SceneComponent.K2_GetComponentToWorld` (`/Game/Blueprints/WaveSpawn/Test/BP_WaveSpawnPoint.Billboard` (`|GetArrayItem` _currentspawnpoint (`KismetMathLibrary.RandomIntegerInRange` 0 (`KismetArrayLibrary.Array_LastIndex` _currentspawnpoint))))) "AdjustIfPossibleButAlwaysSpawn" "OverrideRootScale" null null))
    (`KismetArrayLibrary.Array_Add` (`self.CurrentEnemies`) _returnvalue)))

(fn `UserConstructionScript`)